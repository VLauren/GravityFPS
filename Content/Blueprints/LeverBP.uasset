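; Lever that toggles every BasicDoorBP sharing its Id open or closed, in a game run by GravityGameModeBP.
; Each Tick it registers itself as the player's Lever within a short range and clears that reference outside it.
; Press calls Action, which flips between Activate and Inactivate, moving the button cube whenever a matching door is found.
; With Timer set, further toggles are blocked for TimerTime, then the lever toggles back automatically.
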(event `self.ReceiveTick`
  (params (DeltaSeconds :type "Float (single-precision)"))
  (bind _asgravity_game_mode_bp (cast `/Game/Blueprints/GravityGameModeBP` (`GameplayStatics.GetGameMode`)))
  (bind _player (`/Game/Blueprints/GravityGameModeBP.GetPlayer` _asgravity_game_mode_bp))
  (if (< (`KismetMathLibrary.Vector_Distance` (`self.K2_GetActorLocation` _player) (`self.K2_GetActorLocation`)) 200.0)
    (set `/Game/Blueprints/FirstPersonBP/Blueprints/FirstPersonCharacter.Lever` self _player)
    (elif (== (`/Game/Blueprints/FirstPersonBP/Blueprints/FirstPersonCharacter.Lever` _player) self)
      (set `/Game/Blueprints/FirstPersonBP/Blueprints/FirstPersonCharacter.Lever` null _player))))

(event `Press`
  (`self.Action`)
  (if (`self.Timer`)
    (set `self.TimerActive` true)
    (`KismetSystemLibrary.Delay` (`self.TimerTime`))
    (set `self.TimerActive` false)
    (`self.Action`)))

(fn `Action`
  (if (not (`self.TimerActive`))
    (if (`self.Activated`)
      (`self.Inactivate`)
      (set `self.Activated` false)
      (else
        (`self.Activate`)
        (set `self.Activated` true)))))

(fn `Activate`
  (bind _outactors (`GameplayStatics.GetAllActorsOfClass` "/Game/Blueprints/BasicDoorBP.BasicDoorBP_C"))
  (for _array_element _outactors
    (if (== (`self.id`) (`/Game/Blueprints/BasicDoorBP.id` _array_element))
      (`/Game/Blueprints/BasicDoorBP.Open` _array_element)
      (`SceneComponent.K2_SetRelativeLocation` (`self.CubeBoton`) (-10.0 0.0 0.0) false false))))

(fn `Inactivate`
  (bind _outactors (`GameplayStatics.GetAllActorsOfClass` "/Game/Blueprints/BasicDoorBP.BasicDoorBP_C"))
  (for _array_element _outactors
    (if (== (`self.id`) (`/Game/Blueprints/BasicDoorBP.id` _array_element))
      (`/Game/Blueprints/BasicDoorBP.Close` _array_element)
      (`SceneComponent.K2_SetRelativeLocation` (`self.CubeBoton`) (0.0 0.0 0.0) false false))))

(fn `UserConstructionScript`)