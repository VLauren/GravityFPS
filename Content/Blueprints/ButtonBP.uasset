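; ButtonBP is a pressure-style button that controls doors sharing its Id.
; When an actor begins overlapping it, it finds every BasicDoorBP in the level and opens those with a matching Id.
; When an actor stops overlapping, it closes the same matching doors.
; Both events also print the overlapping actor's name on screen for debugging.
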(event `self.ReceiveActorBeginOverlap`
  (params (OtherActor :type "Actor Object Reference"))
  (`KismetSystemLibrary.PrintString` (`KismetStringLibrary.Concat_StrStr` "Soltar: " (`KismetSystemLibrary.GetDisplayName` OtherActor)) true true (struct :`G` 1.0 :`B` 0.002892 :`A` 1.0))
  (bind _outactors (`GameplayStatics.GetAllActorsOfClass` "/Game/Blueprints/BasicDoorBP.BasicDoorBP_C"))
  (for _array_element _outactors
    (if (== (`self.id`) (`/Game/Blueprints/BasicDoorBP.id` _array_element))
      (`/Game/Blueprints/BasicDoorBP.Open` _array_element))))

(event `self.ReceiveActorEndOverlap`
  (params (OtherActor :type "Actor Object Reference"))
  (`KismetSystemLibrary.PrintString` (`KismetStringLibrary.Concat_StrStr` "Pulsar: " (`KismetSystemLibrary.GetDisplayName` OtherActor)) true true (struct :`R` 0.003097 :`G` 1.0 :`A` 1.0))
  (bind _outactors (`GameplayStatics.GetAllActorsOfClass` "/Game/Blueprints/BasicDoorBP.BasicDoorBP_C"))
  (for _array_element _outactors
    (if (== (`self.id`) (`/Game/Blueprints/BasicDoorBP.id` _array_element))
      (`/Game/Blueprints/BasicDoorBP.Close` _array_element))))

(fn `UserConstructionScript`)