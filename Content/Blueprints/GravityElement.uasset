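; GravityElement is an actor that falls along its own gravity direction, one of six axis directions.
; Each Tick it accelerates and makes a swept move along the vector from GetGravityDirectionVector, independent of engine physics.
; A blocking hit resets velocity and sets CanChangeGravity, which is cleared while it moves freely.
; ShowArrow and HideArrow toggle an arrow component oriented to a supplied direction.
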(event `self.ReceiveTick`
  (params (DeltaSeconds :type "Float (single-precision)"))
  (bind _output_get (set `self.Velocity` (+ (* DeltaSeconds 10.0) (`self.Velocity`))))
  (bind _direction (`self.GetGravityDirectionVector`))
  (bind _sweephitresult (`self.K2_SetActorRelativeLocation` (+ (* _direction _output_get) (`self.K2_GetActorLocation`)) true))
  (if (`GameplayStatics.BreakHitResult` _sweephitresult)
    (set `self.Velocity` 0.1)
    (set `self.CanChangeGravity` true)
    (else
      (set `self.CanChangeGravity` false))))

(fn `GetGravityDirectionVector`
  (returns (Direction :type "Vector Structure"))
  (switch `/Game/Blueprints/GravityDirections` (`self.GravityDirection`)
    (:`NewEnumerator0`
      (return (0.0 0.0 -1.0)))
    (:`NewEnumerator1`
      (return (0.0 0.0 1.0)))
    (:`NewEnumerator2`
      (return (1.0 0.0 0.0)))
    (:`NewEnumerator3`
      (return (-1.0 0.0 0.0)))
    (:`NewEnumerator4`
      (return (0.0 1.0 0.0)))
    (:`NewEnumerator5`
      (return (0.0 -1.0 0.0)))))

(fn `HideArrow`
  (`SceneComponent.SetHiddenInGame` (`self.Arrow`) true false))

(fn `ShowArrow`
  (params (Direction :type "/Game/Blueprints/GravityDirections Enum" :default "NewEnumerator0"))
  (bind _arrow (`self.Arrow`))
  (`SceneComponent.SetHiddenInGame` _arrow false false)
  (`SceneComponent.K2_SetRelativeRotation` _arrow (`KismetMathLibrary.Conv_VectorToRotator` (select `/Game/Blueprints/GravityDirections` Direction :`NewEnumerator0` (0.0 0.0 -1.0) :`NewEnumerator1` (0.0 0.0 1.0) :`NewEnumerator2` (1.0 0.0 0.0) :`NewEnumerator3` (-1.0 0.0 0.0) :`NewEnumerator4` (0.0 1.0 0.0) :`NewEnumerator5` (0.0 -1.0 0.0) :!type "Vector Structure")) false false))

(fn `UserConstructionScript`)